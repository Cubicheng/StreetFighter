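; Player controller for a fighting game that handles the move from menu to character select and each player's selection input.
; The first key press, in the initial game state, blends the view to the "SelectCamera"-tagged actor and brackets the delayed transition with game mode begin/end calls.
; SetImc caches the player index and adds an Enhanced Input context.
; Move and confirm actions forward that index to the select widget.
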(event `Key|AnyKey`
  (params (Key :type "Key Structure"))
  (:`Pressed`
    (`/Engine/EditorBlueprintResources/StandardMacros.DoOnce` false
      (:`Completed`
        (bind _asbp_fighting_game_mode (cast `/Game/_Game/Blueprints/GameModes/BP_FightingGameMode` (`GameplayStatics.GetGameMode`)))
        (bind _output_get (set `self.Fighting Game Mode` _asbp_fighting_game_mode))
        (if (`|EnumEquality` (`/Game/_Game/Blueprints/GameModes/BP_FightingGameMode.E_GameState` _output_get) "NewEnumerator0")
          (bind _outactors (`GameplayStatics.GetAllActorsWithTag` "SelectCamera"))
          (`self.SetViewTargetWithBlend` (`|GetArrayItem` _outactors) (`self.Menu2SelectBlendTime`) "VTBlend_Cubic" 3.0)
          (`/Game/_Game/Blueprints/GameModes/BP_FightingGameMode.Change2SelectBegin` (`self.Fighting Game Mode`))
          (`KismetSystemLibrary.Delay` (`self.Menu2SelectBlendTime`))
          (`/Game/_Game/Blueprints/GameModes/BP_FightingGameMode.Change2SelectEnd` (`self.Fighting Game Mode`)))))))

(event `SetImc`
  (params (IMC :type "InputMappingContext Object Reference"))
  (set `self.PlayerIndex` (`GameplayStatics.GetPlayerControllerID` self))
  (`EnhancedInputSubsystemInterface.AddMappingContext` (subsystem `EnhancedInputLocalPlayerSubsystem`) IMC 0 (struct))
  (`WidgetBlueprintLibrary.SetInputMode_GameAndUIEx` self null))

(event `EnhancedInput|/Game/Input/SelectLevel/Actions/IA_SelectMove`
  (params (ActionValue :type "Float (double-precision)") (ElapsedSeconds :type "Float (double-precision)") (TriggeredSeconds :type "Float (double-precision)") (InputAction :type "InputAction Object Reference" :default "/Game/Input/SelectLevel/Actions/IA_SelectMove.IA_SelectMove"))
  (:`Started`
    (`/Game/_Game/Blueprints/UI/WBP_CharacterSelect.IndexChange` (`self.WBP Character Select`) (select `bool` (> ActionValue 0.0) :`false` -1 :`true` 1) (`self.PlayerIndex`))))

(event `EnhancedInput|/Game/Input/SelectLevel/Actions/IA_Confirm`
  (params (ActionValue :type Boolean) (ElapsedSeconds :type "Float (double-precision)") (TriggeredSeconds :type "Float (double-precision)") (InputAction :type "InputAction Object Reference" :default "/Game/Input/SelectLevel/Actions/IA_Confirm.IA_Confirm"))
  (:`Started`
    (`/Game/_Game/Blueprints/UI/WBP_CharacterSelect.Ready` (`self.WBP Character Select`) (`self.PlayerIndex`))))

(fn `UserConstructionScript`)