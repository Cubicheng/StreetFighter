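; BP_FightGameInstance is the fighting game's game instance, holding each player's character selection.
; GetCharacterBP resolves a player's entry in SelectIndexList to a character Blueprint from CharacterList.
; ChangeCharacterIndex stores the new index for that player, then has BP_FightingGameMode spawn the resolved character, provided that game mode is active.
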(fn `ChangeCharacterIndex`
  (params (CharacterIndex :type Integer) (PlayerIndex :type Integer))
  (`KismetArrayLibrary.Array_Set` (`self.SelectIndexList`) PlayerIndex CharacterIndex)
  (bind _asbp_fighting_game_mode (cast `/Game/_Game/Blueprints/BP_FightingGameMode` (`GameplayStatics.GetGameMode`)))
  (bind _character (`self.GetCharacterBP` PlayerIndex))
  (`/Game/_Game/Blueprints/BP_FightingGameMode.SpawnCharacterBP` _asbp_fighting_game_mode _character PlayerIndex))

(fn `GetCharacterBP`
  (params (PlayerIndex :type Integer))
  (returns (Character :type "/Game/_Game/Blueprints/Characters/BP_BaseCharacter Class Reference"))
  (return (`|GetArrayItem` (`self.CharacterList`) (`|GetArrayItem` (`self.SelectIndexList`) PlayerIndex))))