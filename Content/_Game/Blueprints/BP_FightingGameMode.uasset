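; Game mode for a local two-player fighting game that drives the menu, character select, fight and victory flow.
; It finds tagged menu, select and fight cine cameras, blends both controllers between them, and swaps a widget per phase.
; Selection spawns both fighters and assigns per-player input contexts; fighting possesses them after a countdown and links them as opponents.
; A death shows the winner with win and lose montages, then returns to character select.
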(event `self.ReceiveBeginPlay`
  (set `self.E_GameState` "NewEnumerator0")
  (bind _outactors (`GameplayStatics.GetAllActorsWithTag` "MenuCamera"))
  (bind _ascine_camera_actor (cast `CineCameraActor` (`|GetArrayItem` _outactors)))
  (set `self.MenuCamera` _ascine_camera_actor)
  (bind _outactors_2 (`GameplayStatics.GetAllActorsWithTag` "SelectCamera"))
  (bind _ascine_camera_actor_2 (cast `CineCameraActor` (`|GetArrayItem` _outactors_2)))
  (set `self.SelectCamera` _ascine_camera_actor_2)
  (bind _outactors_3 (`GameplayStatics.GetAllActorsWithTag` "BP_FightCineCamera"))
  (bind _asbp_fight_cine_camera (cast `/Game/_Game/Blueprints/BP_FightCineCamera` (`|GetArrayItem` _outactors_3)))
  (set `self.BP Fight Cine Camera` _asbp_fight_cine_camera)
  (`GameplayStatics.CreatePlayer` 1)
  (`self.SetCamera` 0.0 (`self.MenuCamera`))
  (bind _returnvalue (`|CreateWidget` "/Game/_Game/Blueprints/UI/WBP_Menu.WBP_Menu_C"))
  (`UserWidget.AddToViewport` _returnvalue 0))

(event `Change2SelectBegin`
  (`WidgetLayoutLibrary.RemoveAllWidgets`)
  (set `self.E_GameState` "NewEnumerator1")
  (bind _returnvalue (`|CreateWidget` "/Game/_Game/Blueprints/UI/WBP_CharacterSelect.WBP_CharacterSelect_C"))
  (set `self.WBP_CharacterSelect` _returnvalue)
  (`self.SpawnCharacterBP` "/Game/_Game/Blueprints/Characters/Ninja/BP_NinjaCharacter.BP_NinjaCharacter_C")
  (`self.SpawnCharacterBP` "/Game/_Game/Blueprints/Characters/Ninja/BP_NinjaCharacter.BP_NinjaCharacter_C" 1))

(event `Change2SelectEnd`
  (`UserWidget.AddToViewport` (`self.WBP_CharacterSelect`) 0)
  (bind _asbp_fighting_controller (cast `/Game/_Game/Blueprints/BP_FightingController` (`GameplayStatics.GetPlayerController` 0)))
  (set `/Game/_Game/Blueprints/BP_FightingController.WBP Character Select` (`self.WBP_CharacterSelect`) _asbp_fighting_controller)
  (`/Game/_Game/Blueprints/BP_FightingController.SetImc` _asbp_fighting_controller "/Game/Input/SelectLevel/IMC_SelectPlayer0.IMC_SelectPlayer0")
  (bind _asbp_fighting_controller_2 (cast `/Game/_Game/Blueprints/BP_FightingController` (`GameplayStatics.GetPlayerController` 1)))
  (set `/Game/_Game/Blueprints/BP_FightingController.WBP Character Select` (`self.WBP_CharacterSelect`) _asbp_fighting_controller_2)
  (`/Game/_Game/Blueprints/BP_FightingController.SetImc` _asbp_fighting_controller_2 "/Game/Input/SelectLevel/IMC_SelectPlayer1.IMC_SelectPlayer1"))

(event `Change2Fighting`
  (bind _returnvalue (`GameplayStatics.GetPlayerController` 0))
  (bind _returnvalue_2 (`GameplayStatics.GetPlayerController` 1))
  (bind _playerlist (`self.PlayerList`))
  (bind _playerlist_2 (`self.PlayerList`))
  (`WidgetLayoutLibrary.RemoveAllWidgets`)
  (set `self.E_GameState` "NewEnumerator2")
  (`/Game/_Game/Blueprints/BP_FightCineCamera.OnEnterFight` (`self.BP Fight Cine Camera`))
  (`self.SetCamera` 0.0 (`self.SelectCamera`))
  (`self.SetFightCamera` 3.0)
  (bind _returnvalue_3 (`|CreateWidget` "/Game/_Game/Blueprints/UI/WBP_CountDown.WBP_CountDown_C"))
  (`UserWidget.AddToViewport` _returnvalue_3 0)
  (`KismetSystemLibrary.Delay` 4.0)
  (`Controller.Possess` _returnvalue (`|GetArrayItem` (`self.PlayerList`)))
  (`EnhancedInputSubsystemInterface.AddMappingContext` (pcsubsystem `EnhancedInputLocalPlayerSubsystem` _returnvalue) "/Game/Input/FightLevel/IMC_Player0.IMC_Player0" 0 (struct))
  (`Controller.Possess` _returnvalue_2 (`|GetArrayItem` (`self.PlayerList`) 1))
  (`EnhancedInputSubsystemInterface.AddMappingContext` (pcsubsystem `EnhancedInputLocalPlayerSubsystem` _returnvalue_2) "/Game/Input/FightLevel/IMC_Player1.IMC_Player1" 0 (struct))
  (set `/Game/_Game/Blueprints/Characters/BP_BaseCharacter.Opponent` (`|GetArrayItem` _playerlist_2 1) (`|GetArrayItem` _playerlist_2))
  (set `/Game/_Game/Blueprints/Characters/BP_BaseCharacter.Opponent` (`|GetArrayItem` _playerlist) (`|GetArrayItem` _playerlist 1))
  (`self.SetFightCamera` 0.0)
  (bind _returnvalue_4 (`|CreateWidget` "/Game/_Game/Blueprints/UI/WBP_FightingUI.WBP_FightingUI_C"))
  (`UserWidget.AddToViewport` _returnvalue_4 0))

(event `OnPlayerDied`
  (params (DeadPlayerIndex :type Integer))
  (bind _output_get (set `self.DeadPlayerIndex` DeadPlayerIndex))
  (set `self.WinPlayerIndex` (`KismetMathLibrary.Xor_IntInt` _output_get 1))
  (set `self.IsGameOver` true)
  (`WidgetBlueprintLibrary.SetInputMode_UIOnlyEx` (`GameplayStatics.GetPlayerController` 0) null)
  (`WidgetBlueprintLibrary.SetInputMode_UIOnlyEx` (`GameplayStatics.GetPlayerController` 1) null)
  (bind _returnvalue (`|CreateWidget` "/Game/_Game/Blueprints/UI/WBP_WinningUI.WBP_WinningUI_C" null (`self.WinPlayerIndex`)))
  (`UserWidget.AddToViewport` _returnvalue 0)
  (`/Game/_Game/Blueprints/Characters/BP_BaseCharacter.PlayLoseMontage` (`|GetArrayItem` (`self.PlayerList`) (`self.DeadPlayerIndex`)))
  (`/Game/_Game/Blueprints/Characters/BP_BaseCharacter.PlayWinMontage` (`|GetArrayItem` (`self.PlayerList`) (`self.WinPlayerIndex`))))

(event `OnVictoryAnimEnd`
  (set `self.E_GameState` "NewEnumerator1")
  (`WidgetLayoutLibrary.RemoveAllWidgets`)
  (`self.K2_DestroyActor` (`|GetArrayItem` (`self.PlayerList`)))
  (`self.K2_DestroyActor` (`|GetArrayItem` (`self.PlayerList`) 1))
  (`self.Change2SelectBegin`)
  (`self.SetFightCamera` 0.0)
  (`self.SetCamera` 3.0 (`self.SelectCamera`))
  (`self.Change2SelectEnd`))

(fn `SetCamera`
  (params (`Blend Time` :type "Float (double-precision)") (Camera :type "CineCameraActor Object Reference"))
  (`PlayerController.SetViewTargetWithBlend` (`GameplayStatics.GetPlayerController` 0) Camera `Blend Time` "VTBlend_Linear" 3.0 false)
  (`PlayerController.SetViewTargetWithBlend` (`GameplayStatics.GetPlayerController` 1) Camera `Blend Time` "VTBlend_Linear" 3.0 false))

(fn `SetFightCamera`
  (params (BlendTime :type "Float (double-precision)"))
  (`PlayerController.SetViewTargetWithBlend` (`GameplayStatics.GetPlayerController` 0) (`self.BP Fight Cine Camera`) BlendTime "VTBlend_Linear" 3.0 false)
  (`PlayerController.SetViewTargetWithBlend` (`GameplayStatics.GetPlayerController` 1) (`self.BP Fight Cine Camera`) BlendTime "VTBlend_Linear" 3.0 false))

(fn `SpawnCharacterBP`
  (params (Character :type "/Game/_Game/Blueprints/Characters/BP_BaseCharacter Class Reference") (PlayerIndex :type Integer))
  (bind _output (`|GetArrayItem` (`self.PlayerList`) PlayerIndex))
  (if (`KismetSystemLibrary.IsValid` _output)
    (`self.K2_DestroyActor` _output))
  (bind _returnvalue (`|SpawnActorFromClass` Character (`|GetArrayItem` (`self.PlayerSpawnTransformList`) PlayerIndex) "AdjustIfPossibleButAlwaysSpawn" "MultiplyWithRoot" null PlayerIndex null))
  (`KismetArrayLibrary.Array_Set` (`self.PlayerList`) PlayerIndex _returnvalue))

(fn `UserConstructionScript`)