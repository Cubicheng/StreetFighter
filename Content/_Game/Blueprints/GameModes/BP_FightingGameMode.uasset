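; Game mode for a local two-player fighting game, driving the flow from menu through character select to fight and win screen.
; Character select spawns default ninjas via a respawn helper and gives each controller its own input context.
; Fight start possesses both characters, links them as opponents and blends between tagged cameras.
; A death disables input, shows the winner UI and plays win and lose montages.
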(event `self.ReceiveBeginPlay`
  (set `self.E_GameState` "NewEnumerator0")
  (`GameplayStatics.CreatePlayer` 1)
  (`self.SetCamera` "MenuCamera"))

(event `Change2SelectBegin`
  (set `self.E_GameState` "NewEnumerator1")
  (bind _returnvalue (`|CreateWidget` "/Game/_Game/Blueprints/UI/WBP_CharacterSelect.WBP_CharacterSelect_C"))
  (set `self.WBP_CharacterSelect` _returnvalue)
  (`self.SpawnCharacterBP` "/Game/_Game/Blueprints/Characters/Ninja/BP_NinjaCharacter.BP_NinjaCharacter_C")
  (`self.SpawnCharacterBP` "/Game/_Game/Blueprints/Characters/Ninja/BP_NinjaCharacter.BP_NinjaCharacter_C" 1))

(event `Change2SelectEnd`
  (`UserWidget.AddToViewport` (`self.WBP_CharacterSelect`) 0)
  (bind _asbp_fighting_controller (cast `/Game/_Game/Blueprints/Controllers/BP_FightingController` (`GameplayStatics.GetPlayerController` 0)))
  (set `/Game/_Game/Blueprints/Controllers/BP_FightingController.WBP Character Select` (`self.WBP_CharacterSelect`) _asbp_fighting_controller)
  (`/Game/_Game/Blueprints/Controllers/BP_FightingController.SetImc` _asbp_fighting_controller "/Game/Input/SelectLevel/IMC_SelectPlayer0.IMC_SelectPlayer0")
  (bind _asbp_fighting_controller_2 (cast `/Game/_Game/Blueprints/Controllers/BP_FightingController` (`GameplayStatics.GetPlayerController` 1)))
  (set `/Game/_Game/Blueprints/Controllers/BP_FightingController.WBP Character Select` (`self.WBP_CharacterSelect`) _asbp_fighting_controller_2)
  (`/Game/_Game/Blueprints/Controllers/BP_FightingController.SetImc` _asbp_fighting_controller_2 "/Game/Input/SelectLevel/IMC_SelectPlayer1.IMC_SelectPlayer1"))

(event `SpawnCharacter`
  (params (Index :type Integer)))

(event `Change2Fighting`
  (bind _returnvalue (`GameplayStatics.GetPlayerController` 0))
  (bind _returnvalue_2 (`GameplayStatics.GetPlayerController` 1))
  (bind _playerlist (`self.PlayerList`))
  (bind _playerlist_2 (`self.PlayerList`))
  (`WidgetLayoutLibrary.RemoveAllWidgets`)
  (set `self.E_GameState` "NewEnumerator2")
  (`Controller.Possess` _returnvalue (`|GetArrayItem` (`self.PlayerList`)))
  (`EnhancedInputSubsystemInterface.AddMappingContext` (pcsubsystem `EnhancedInputLocalPlayerSubsystem` _returnvalue) "/Game/Input/FightLevel/IMC_Player0.IMC_Player0" 0 (struct))
  (`Controller.Possess` _returnvalue_2 (`|GetArrayItem` (`self.PlayerList`) 1))
  (`EnhancedInputSubsystemInterface.AddMappingContext` (pcsubsystem `EnhancedInputLocalPlayerSubsystem` _returnvalue_2) "/Game/Input/FightLevel/IMC_Player1.IMC_Player1" 0 (struct))
  (set `/Game/_Game/Blueprints/Characters/BP_BaseCharacter.Opponent` (`|GetArrayItem` _playerlist_2 1) (`|GetArrayItem` _playerlist_2))
  (set `/Game/_Game/Blueprints/Characters/BP_BaseCharacter.Opponent` (`|GetArrayItem` _playerlist) (`|GetArrayItem` _playerlist 1))
  (`self.SetCamera` "SelectCamera" 0.0)
  (`self.SetCamera` "FightCamera" 2.0)
  (bind _returnvalue_3 (`|CreateWidget` "/Game/_Game/Blueprints/UI/WBP_FightingUI.WBP_FightingUI_C"))
  (`UserWidget.AddToViewport` _returnvalue_3 0))

(event `OnPlayerDied`
  (params (DeadPlayerIndex :type Integer))
  (bind _playerlist (`self.PlayerList`))
  (bind _output_get (set `self.DeadPlayerIndex` DeadPlayerIndex))
  (set `self.WinPlayerIndex` (`KismetMathLibrary.Xor_IntInt` _output_get 1))
  (set `self.IsGameOver` true)
  (`self.DisableInput` (`|GetArrayItem` _playerlist) (`GameplayStatics.GetPlayerController` 0))
  (`self.DisableInput` (`|GetArrayItem` _playerlist 1) (`GameplayStatics.GetPlayerController` 1))
  (bind _returnvalue (`|CreateWidget` "/Game/_Game/Blueprints/UI/WBP_WinningUI.WBP_WinningUI_C" null (`self.WinPlayerIndex`)))
  (`UserWidget.AddToViewport` _returnvalue 0)
  (`/Game/_Game/Blueprints/Characters/BP_BaseCharacter.PlayLoseMontage` (`|GetArrayItem` (`self.PlayerList`) (`self.DeadPlayerIndex`)))
  (`/Game/_Game/Blueprints/Characters/BP_BaseCharacter.PlayWinMontage` (`|GetArrayItem` (`self.PlayerList`) (`self.WinPlayerIndex`))))

(fn `SetCamera`
  (params (CameraTag :type Name) (`Blend Time` :type "Float (double-precision)"))
  (bind _outactors (`GameplayStatics.GetAllActorsWithTag` CameraTag))
  (bind _output (`|GetArrayItem` _outactors))
  (`PlayerController.SetViewTargetWithBlend` (`GameplayStatics.GetPlayerController` 0) _output `Blend Time` "VTBlend_Linear" 3.0 false)
  (`PlayerController.SetViewTargetWithBlend` (`GameplayStatics.GetPlayerController` 1) _output `Blend Time` "VTBlend_Linear" 3.0 false))

(fn `SpawnCharacterBP`
  (params (Character :type "/Game/_Game/Blueprints/Characters/BP_BaseCharacter Class Reference") (PlayerIndex :type Integer))
  (bind _output (`|GetArrayItem` (`self.PlayerList`) PlayerIndex))
  (if (`KismetSystemLibrary.IsValid` _output)
    (`self.K2_DestroyActor` _output))
  (bind _returnvalue (`|SpawnActorFromClass` Character (`|GetArrayItem` (`self.PlayerSpawnTransformList`) PlayerIndex) "AdjustIfPossibleButAlwaysSpawn" "MultiplyWithRoot" null PlayerIndex null))
  (`KismetArrayLibrary.Array_Set` (`self.PlayerList`) PlayerIndex _returnvalue))

(fn `UserConstructionScript`)