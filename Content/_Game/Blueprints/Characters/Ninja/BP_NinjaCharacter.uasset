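; Ninja fighter character Blueprint that turns move, jump and block input into montage-driven actions and supplies the ninja's animation set to inherited character logic.
; Movement flips input by facing direction and plays forward or backward step montages while updating CurrentState, with directional movement input applied when falling.
; Blocking costs energy and jumping cancels it.
; Attack events spawn and remove a socket-attached BP_NinjaAttack with normal or super-move damage.
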(event `self.ReceiveBeginPlay`
  (`parent.ReceiveBeginPlay`))

(event `self.ReceiveTick`
  (params (DeltaSeconds :type "Float (single-precision)"))
  (`parent.ReceiveTick` DeltaSeconds))

(event `EnhancedInput|/Game/Input/FightLevel/Actions/IA_Move`
  (params (ActionValue :type "Vector2D Structure") (ElapsedSeconds :type "Float (double-precision)") (TriggeredSeconds :type "Float (double-precision)") (InputAction :type "InputAction Object Reference" :default "/Game/Input/FightLevel/Actions/IA_Move.IA_Move"))
  (:`Triggered`
    (bind _canmove (`self.CanMove`))
    (if _canmove
      (bind _outputx (`self.CalcMoveInputByPlayerIndex` ActionValue_X))
      (bind _output_get (set `self.MoveInput` _outputx))
      (if (`|EnumEquality` (`self.CurrentState`) "NewEnumerator0")
        (set `self.CurrentState` "NewEnumerator1")
        (if (> _output_get 0.0) :!label _label
          (`|PlayMontage` (`self.Mesh`) "/Game/_Game/Assets/Animations/Ninja/Short_Step_Forward_Anim_Montage.Short_Step_Forward_Anim_Montage" 1.5
            (:`OnCompleted`
              _))
          (else
            (`|PlayMontage` (`self.Mesh`) "/Game/_Game/Assets/Animations/Ninja/Step_Backward_Anim_Montage.Step_Backward_Anim_Montage"
              (:`OnCompleted`
                _))))
        (set `self.CurrentState` "NewEnumerator0"))
      (elif (`NavMovementComponent.IsFalling` (`self.CharacterMovement`))
        (`self.AddMovementInput` (1.0 1.0 0.0) ActionValue_X))))
  (:`Started`
    (bind _canmove_2 (`self.CanMove`))
    (if _canmove_2
      (goto _label)))
  (:`Completed`
    (if (`|EnumEquality` (`self.CurrentState`) "NewEnumerator1")
      (`self.StopAnimMontage` "/Game/_Game/Assets/Animations/Ninja/Step_Backward_Anim_Montage.Step_Backward_Anim_Montage")
      (`self.StopAnimMontage` "/Game/_Game/Assets/Animations/Ninja/Short_Step_Forward_Anim_Montage.Short_Step_Forward_Anim_Montage")
      (set `self.CurrentState` "NewEnumerator0"))))

(event `SpawnAttackActor`
  (params (IsSuperMove :type Boolean))
  (bind _returnvalue (`|SpawnActorFromClass` "/Game/_Game/Blueprints/Characters/Ninja/BP_NinjaAttack.BP_NinjaAttack_C" (`SceneComponent.GetSocketTransform` (`self.Mesh`) (`self.AttackSocketName`) "RTS_World") "Undefined" "MultiplyWithRoot" null (select `bool` IsSuperMove :`false` (`self.NormalAttackDamageNum`) :`true` (`self.SuperMoveDamageNum`)) self))
  (bind _output_get (set `self.AttackActor` _returnvalue))
  (`self.K2_AttachToComponent` _output_get (`self.Mesh`) (`self.AttackSocketName`) "SnapToTarget" "SnapToTarget" "SnapToTarget" true))

(event `RemoveAttackActor`
  (`self.K2_DestroyActor` (`self.AttackActor`)))

(event `EnhancedInput|/Game/Input/FightLevel/Actions/IA_Jump`
  (params (ActionValue :type Boolean) (ElapsedSeconds :type "Float (double-precision)") (TriggeredSeconds :type "Float (double-precision)") (InputAction :type "InputAction Object Reference" :default "/Game/Input/FightLevel/Actions/IA_Jump.IA_Jump"))
  (:`Started`
    (bind _canjump (`self.CanChange2Jump`))
    (if _canjump
      (`self.SetIsBlocking` false)
      (set `self.CurrentState` "NewEnumerator4")
      (`self.SetIsBlocking` false)
      (`|PlayMontage` (`self.Mesh`) (`self.JumpMontage`)
        (:`OnCompleted`
          (set `self.CurrentState` "NewEnumerator0"))))))

(event `EnhancedInput|/Game/Input/FightLevel/Actions/IA_Block`
  (params (ActionValue :type Boolean) (ElapsedSeconds :type "Float (double-precision)") (TriggeredSeconds :type "Float (double-precision)") (InputAction :type "InputAction Object Reference" :default "/Game/Input/FightLevel/Actions/IA_Block.IA_Block"))
  (:`Triggered`
    (bind _canblock (`self.CanBlock`))
    (if _canblock
      (`self.SetIsBlocking` true)
      (`self.AddEnergy` (* (`self.ENERGY COST ON BEGIN BLOCK`) -1.0))))
  (:`Completed`
    (`self.SetIsBlocking` false)))

(fn `CalcMoveInputByPlayerIndex`
  (params (inputX :type "Float (double-precision)"))
  (returns (outputX :type "Float (double-precision)"))
  (bind (_returnvalue_x _returnvalue_y) (`KismetMathLibrary.BreakVector` (`self.GetActorForwardVector`)))
  (return (* inputX _returnvalue_y)))

(fn `UserConstructionScript`
  (set `self.JumpMontage` "/Game/_Game/Assets/Animations/Ninja/Jumping_Anim_Montage.Jumping_Anim_Montage")
  (set `self.LightHittedMontage` "/Game/_Game/Assets/Animations/Ninja/Light_Hit_To_Head_Anim_Montage.Light_Hit_To_Head_Anim_Montage")
  (set `self.BigHittedMontage` "/Game/_Game/Assets/Animations/Ninja/Hit_To_Body_Anim_Montage.Hit_To_Body_Anim_Montage")
  (set `self.WinMontage` "/Game/_Game/Assets/Animations/Ninja/Victory_Anim_Montage.Victory_Anim_Montage")
  (set `self.LoseMontage` "/Game/_Game/Assets/Animations/Ninja/Knocked_Out_Anim_Montage.Knocked_Out_Anim_Montage")
  (set `self.AttackMontage` "/Game/_Game/Assets/Animations/Ninja/Boxing_Anim_Montage.Boxing_Anim_Montage")
  (set `self.SuperMoveMontage` "/Game/_Game/Assets/Animations/Ninja/Hook_Anim_Montage.Hook_Anim_Montage"))