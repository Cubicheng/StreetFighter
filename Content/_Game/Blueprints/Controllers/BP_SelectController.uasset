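; Player controller for the two-player character select screen, driving the character select widget for its local player.
; On BeginPlay it reads its controller ID, adds that player's Enhanced Input mapping context and sets Game and UI input mode.
; Move input steps that player's selection left or right by the sign of the value, and confirm marks that player ready on the widget.
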(event `self.ReceiveBeginPlay`
  (set `self.Index` (`GameplayStatics.GetPlayerControllerID` self))
  (`EnhancedInputSubsystemInterface.AddMappingContext` (subsystem `EnhancedInputLocalPlayerSubsystem`) (select `int` (`self.Index`) :`0` "/Game/Input/SelectLevel/IMC_SelectPlayer0.IMC_SelectPlayer0" :`1` "/Game/Input/SelectLevel/IMC_SelectPlayer1.IMC_SelectPlayer1" :!type "InputMappingContext Object Reference") 0 (struct))
  (`WidgetBlueprintLibrary.SetInputMode_GameAndUIEx` self null))

(event `EnhancedInput|/Game/Input/SelectLevel/Actions/IA_SelectMove`
  (params (ActionValue :type "Float (double-precision)") (ElapsedSeconds :type "Float (double-precision)") (TriggeredSeconds :type "Float (double-precision)") (InputAction :type "InputAction Object Reference" :default "/Game/Input/SelectLevel/Actions/IA_SelectMove.IA_SelectMove"))
  (bind _wbp_characterselect (`self.WBP_CharacterSelect`))
  (bind _returnvalue (select `bool` (> ActionValue 0.0) :`false` -1 :`true` 1))
  (:`Started`
    (if (== (`self.Index`) 0)
      (`/Game/_Game/Blueprints/UI/WBP_CharacterSelect.P0IndexChange` _wbp_characterselect _returnvalue)
      (else
        (`/Game/_Game/Blueprints/UI/WBP_CharacterSelect.P1IndexChanged` _wbp_characterselect _returnvalue)))))

(event `EnhancedInput|/Game/Input/SelectLevel/Actions/IA_Confirm`
  (params (ActionValue :type Boolean) (ElapsedSeconds :type "Float (double-precision)") (TriggeredSeconds :type "Float (double-precision)") (InputAction :type "InputAction Object Reference" :default "/Game/Input/SelectLevel/Actions/IA_Confirm.IA_Confirm"))
  (bind _wbp_characterselect (`self.WBP_CharacterSelect`))
  (:`Started`
    (if (== (`self.Index`) 0)
      (`/Game/_Game/Blueprints/UI/WBP_CharacterSelect.P0Ready` _wbp_characterselect)
      (else
        (`/Game/_Game/Blueprints/UI/WBP_CharacterSelect.P1Ready` _wbp_characterselect)))))

(fn `UserConstructionScript`)