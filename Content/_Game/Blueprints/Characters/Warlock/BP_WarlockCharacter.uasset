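; Playable Warlock fighter Blueprint that adds fireball attacks and an energy-gated super move to its parent character.
; Enhanced Input drives movement, jump, block and super move, using state checks, montages and energy costs.
; Separate events spawn a socket-attached fireball, launch it, toggle a Niagara charge effect and spawn the super attack ahead of the character.
; The construction script assigns Warlock-specific montages to the character's animation slots.
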(event `self.ReceiveBeginPlay`
  (`parent.ReceiveBeginPlay`))

(event `self.ReceiveTick`
  (params (DeltaSeconds :type "Float (single-precision)"))
  (`parent.ReceiveTick` DeltaSeconds))

(event `EnhancedInput|/Game/Input/FightLevel/Actions/IA_Move`
  (params (ActionValue :type "Vector2D Structure") (ElapsedSeconds :type "Float (double-precision)") (TriggeredSeconds :type "Float (double-precision)") (InputAction :type "InputAction Object Reference" :default "/Game/Input/FightLevel/Actions/IA_Move.IA_Move"))
  (:`Triggered`
    (bind _canmove (`self.CanMove`))
    (if _canmove
      (`self.AddMovementInput` (1.0 1.0 1.0) ActionValue_X)
      (set `self.CurrentState` "NewEnumerator1")
      (if (<= ActionValue_X 0.0)
        _)
      (elif (`NavMovementComponent.IsFalling` (`self.CharacterMovement`))
        (`self.AddMovementInput` (1.0 1.0 0.0) ActionValue_X))))
  (:`Completed`
    (if (`|EnumEquality` (`self.CurrentState`) "NewEnumerator1")
      (set `self.CurrentState` "NewEnumerator0"))))

(event `SpawnAttackFireBall`
  (bind _returnvalue_location (`KismetMathLibrary.BreakTransform` (`SceneComponent.GetSocketTransform` (`self.Mesh`) (`self.FireballSocketName`) "RTS_World")))
  (bind _returnvalue (`|SpawnActorFromClass` "/Game/_Game/Blueprints/Characters/Warlock/BP_Fireball.BP_Fireball_C" (`KismetMathLibrary.MakeTransform` _returnvalue_location) "Undefined" "MultiplyWithRoot" null (`self.NormalAttackDamageNum`) self))
  (bind _output_get (set `self.CurrentFireball` _returnvalue))
  (`self.K2_AttachToComponent` _output_get (`self.Mesh`) (`self.FireballSocketName`) "SnapToTarget" "SnapToTarget" "KeepWorld" true))

(event `LaunchFireball`
  (`/Game/_Game/Blueprints/Characters/Warlock/BP_Fireball.LaunchFireball` (`self.CurrentFireball`)))

(event `EnhancedInput|/Game/Input/FightLevel/Actions/IA_SuperMove`
  (params (ActionValue :type Boolean) (ElapsedSeconds :type "Float (double-precision)") (TriggeredSeconds :type "Float (double-precision)") (InputAction :type "InputAction Object Reference" :default "/Game/Input/FightLevel/Actions/IA_SuperMove.IA_SuperMove"))
  (:`Started`
    (if (>= (`self.Energy`) (`self.MaxEnergy`))
      (bind _canattack (`self.CanAttack`))
      (if _canattack
        (`self.SetIsBlocking` false)
        (set `self.Energy` 0.0)
        (set `self.CurrentState` "NewEnumerator2")
        (`self.SetIsBlocking` false)
        (`|PlayMontage` (`self.Mesh`) "/Game/_Game/Assets/Animations/Warlock/Standing_2H_Magic_Area_Attack_02_Anim_Montage.Standing_2H_Magic_Area_Attack_02_Anim_Montage"
          (:`OnCompleted`
            (set `self.CurrentState` "NewEnumerator0")))))))

(event `SpawnSuperMoveAttack`
  (bind _supermoveoffset (`self.GetSuperMoveOffset`))
  (`|SpawnActorFromClass` "/Game/_Game/Blueprints/Characters/Warlock/BP_SuperMoveAttack.BP_SuperMoveAttack_C" (`KismetMathLibrary.MakeTransform` _supermoveoffset) "Undefined" "MultiplyWithRoot" null (`self.SuperMoveDamageNum`) self))

(event `SpawnChargeEffect`
  (bind _supermoveoffset (`self.GetSuperMoveOffset`))
  (bind _returnvalue (`NiagaraFunctionLibrary.SpawnSystemAtLocation` "/Game/_Game/Assets/Characters/Warlock/FX/NS_MagicBall.NS_MagicBall" _supermoveoffset))
  (set `self.ChargeEffect` _returnvalue))

(event `RemoveChargeEffect`
  (`ActorComponent.K2_DestroyComponent` (`self.ChargeEffect`)))

(event `EnhancedInput|/Game/Input/FightLevel/Actions/IA_Jump`
  (params (ActionValue :type Boolean) (ElapsedSeconds :type "Float (double-precision)") (TriggeredSeconds :type "Float (double-precision)") (InputAction :type "InputAction Object Reference" :default "/Game/Input/FightLevel/Actions/IA_Jump.IA_Jump"))
  (:`Started`
    (bind _canjump (`self.CanChange2Jump`))
    (if _canjump
      (`self.SetIsBlocking` false)
      (set `self.CurrentState` "NewEnumerator4")
      (`self.SetIsBlocking` false)
      (`|PlayMontage` (`self.Mesh`) (`self.JumpMontage`)
        (:`OnCompleted`
          (set `self.CurrentState` "NewEnumerator0"))))))

(event `EnhancedInput|/Game/Input/FightLevel/Actions/IA_Block`
  (params (ActionValue :type Boolean) (ElapsedSeconds :type "Float (double-precision)") (TriggeredSeconds :type "Float (double-precision)") (InputAction :type "InputAction Object Reference" :default "/Game/Input/FightLevel/Actions/IA_Block.IA_Block"))
  (:`Triggered`
    (bind _canblock (`self.CanBlock`))
    (if _canblock
      (`self.SetIsBlocking` true)
      (`self.AddEnergy` (* (`self.ENERGY COST ON BEGIN BLOCK`) -1.0))))
  (:`Completed`
    (`self.SetIsBlocking` false)))

(fn `GetSuperMoveOffset`
  (returns (SuperMoveOffset :type "Vector Structure"))
  (return (+ (+ (`self.K2_GetActorLocation`) (* (`self.GetActorForwardVector`) (`self.SuperMoveForwardOffset`))) (* (`self.GetActorUpVector`) (`self.SuperMoveUpOffset`)))))

(fn `UserConstructionScript`
  (set `self.JumpMontage` "/Game/_Game/Assets/Animations/Warlock/Standing_Jump_Anim_Montage.Standing_Jump_Anim_Montage")
  (set `self.LightHittedMontage` "/Game/_Game/Assets/Animations/Warlock/Standing_React_Small_From_Front_Anim_Montage.Standing_React_Small_From_Front_Anim_Montage")
  (set `self.BigHittedMontage` "/Game/_Game/Assets/Animations/Warlock/Standing_React_Large_From_Front_Anim_Montage.Standing_React_Large_From_Front_Anim_Montage")
  (set `self.WinMontage` "/Game/_Game/Assets/Animations/Warlock/Victory_Anim_Montage.Victory_Anim_Montage")
  (set `self.LoseMontage` "/Game/_Game/Assets/Animations/Warlock/Standing_React_Death_Backward_Anim_Montage.Standing_React_Death_Backward_Anim_Montage")
  (set `self.AttackMontage` "/Game/_Game/Assets/Animations/Warlock/Standing_1H_Magic_Attack_01_Anim_Montage.Standing_1H_Magic_Attack_01_Anim_Montage")
  (set `self.SuperMoveMontage` "/Game/_Game/Assets/Animations/Warlock/Standing_2H_Magic_Area_Attack_02_Anim_Montage.Standing_2H_Magic_Area_Attack_02_Anim_Montage"))