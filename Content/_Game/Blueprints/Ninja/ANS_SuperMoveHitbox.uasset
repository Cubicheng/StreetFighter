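; Anim notify state that acts as the super move attack hitbox on an animated character.
; On begin it clears the owning BP_BaseCharacter's hit list.
; Each tick it spawns the super move Niagara effect at a socket and sphere-traces there for pawns, with debug drawing.
; Hits accepted by RegisterHitActor call OnHitted on the victim with the attack number, then OnHit on the attacker with the victim's blocking state.
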(fn `Received_NotifyBegin`
  (params (MeshComp :type "SkeletalMeshComponent Object Reference") (Animation :type "AnimSequenceBase Object Reference") (TotalDuration :type "Float (single-precision)") (EventReference :type "AnimNotifyEventReference Structure (by ref)"))
  (returns (ReturnValue :type Boolean))
  (bind _asbp_base_character (cast `/Game/_Game/Blueprints/BP_BaseCharacter` (`ActorComponent.GetOwner` MeshComp)))
  (`KismetArrayLibrary.Array_Clear` (`/Game/_Game/Blueprints/BP_BaseCharacter.HitActorList` _asbp_base_character))
  (return false))

(fn `Received_NotifyTick`
  (params (MeshComp :type "SkeletalMeshComponent Object Reference") (Animation :type "AnimSequenceBase Object Reference") (FrameDeltaTime :type "Float (single-precision)") (EventReference :type "AnimNotifyEventReference Structure (by ref)"))
  (returns (ReturnValue :type Boolean))
  (bind _returnvalue (`SceneComponent.GetSocketLocation` MeshComp (`self.SocketName`)))
  (`NiagaraFunctionLibrary.SpawnSystemAttached` "/Game/_Game/Assets/Characters/Ninja/FX/NS_SuperMove_VFX.NS_SuperMove_VFX" MeshComp (`self.SocketName`) (0.0 0.0 0.0) (struct) "KeepRelativeOffset")
  (bind _outhit (`KismetSystemLibrary.SphereTraceSingleForObjects` :`WorldContextObject` MeshComp :`Start` _returnvalue :`End` _returnvalue :`Radius` 20.0 :`ObjectTypes` (`|MakeArray` "ObjectTypeQuery3" :!type "EObjectTypeQuery Enum") :`DrawDebugType` "ForOneFrame"))
  (bind _asbp_base_character (cast `/Game/_Game/Blueprints/BP_BaseCharacter` (`.HitActor` (`GameplayStatics.BreakHitResult` _outhit))))
  (bind _asbp_base_character_2 (cast `/Game/_Game/Blueprints/BP_BaseCharacter` (`ActorComponent.GetOwner` MeshComp)))
  (bind _isnewhit (`/Game/_Game/Blueprints/BP_BaseCharacter.RegisterHitActor` _asbp_base_character_2 _asbp_base_character))
  (if _isnewhit
    (`/Game/_Game/Blueprints/BP_BaseCharacter.OnHitted` _asbp_base_character (`self.SuperMoveAttackNum`))
    (`/Game/_Game/Blueprints/BP_BaseCharacter.OnHit` _asbp_base_character_2 (`/Game/_Game/Blueprints/BP_BaseCharacter.IsBlocking` _asbp_base_character))
    (return false)))