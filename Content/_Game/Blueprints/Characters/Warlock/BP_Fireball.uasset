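; BP_Fireball is a Warlock projectile that damages the first character it touches other than its instigator.
; LaunchFireball detaches it in world space and sets ProjectileMovement velocity along the instigator's forward vector at Speed.
; On Sphere overlap with a BP_BaseCharacter, it calls OnHitted with the damage, destroys itself, then reports the victim's blocking state to the instigator through OnHit.
; Overlaps with non-character actors leave it intact.
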(event `LaunchFireball`
  (`self.K2_DetachFromActor` "KeepWorld" "KeepWorld" "KeepWorld")
  (set `MovementComponent.Velocity` (* (`self.GetActorForwardVector` (`self.GetInstigator`)) (`self.Speed`)) (`self.ProjectileMovement`)))

(event `self.Sphere.OnComponentBeginOverlap`
  (params (OverlappedComponent :type "PrimitiveComponent Object Reference") (OtherActor :type "Actor Object Reference") (OtherComp :type "PrimitiveComponent Object Reference") (OtherBodyIndex :type Integer) (bFromSweep :type Boolean) (SweepResult :type "HitResult Structure (by ref)"))
  (bind _returnvalue (`self.GetInstigator`))
  (if (!= OtherActor _returnvalue)
    (bind _asbp_base_character (cast `/Game/_Game/Blueprints/Characters/BP_BaseCharacter` OtherActor))
    (`/Game/_Game/Blueprints/Characters/BP_BaseCharacter.OnHitted` _asbp_base_character (`self.FireballDamageNum`))
    (`self.K2_DestroyActor`)
    (bind _asbp_base_character_2 (cast `/Game/_Game/Blueprints/Characters/BP_BaseCharacter` _returnvalue))
    (`/Game/_Game/Blueprints/Characters/BP_BaseCharacter.OnHit` _asbp_base_character_2 (`/Game/_Game/Blueprints/Characters/BP_BaseCharacter.IsBlocking` _asbp_base_character))))

(fn `UserConstructionScript`)