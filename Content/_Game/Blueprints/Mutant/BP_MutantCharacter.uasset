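; BP_MutantCharacter is the playable Mutant fighter, built on a parent class and configured with its own reaction, win, lose and attack montages in the construction script.
; Enhanced Input movement, gated by CanMove, applies one-axis input and updates CurrentState.
; SpawnAttackActor creates a BP_MutantNormalAttack with normal or super-move damage, always attaching it to the mesh's normal attack socket.
; RemoveAttackActor destroys that attack actor.
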(event `self.ReceiveBeginPlay`
  (`parent.ReceiveBeginPlay`))

(event `self.ReceiveTick`
  (params (DeltaSeconds :type "Float (single-precision)"))
  (`parent.ReceiveTick` DeltaSeconds))

(event `EnhancedInput|/Game/Input/Actions/IA_Move`
  (params (ActionValue :type "Vector2D Structure") (ElapsedSeconds :type "Float (double-precision)") (TriggeredSeconds :type "Float (double-precision)") (InputAction :type "InputAction Object Reference" :default "/Game/Input/Actions/IA_Move.IA_Move"))
  (:`Triggered`
    (bind _canmove (`self.CanMove`))
    (if _canmove
      (`self.AddMovementInput` (1.0 1.0 1.0) ActionValue_X)
      (set `self.CurrentState` "NewEnumerator1")
      (if (<= ActionValue_X 0.0)
        _)))
  (:`Completed`
    (if (`|EnumEquality` (`self.CurrentState`) "NewEnumerator1")
      (set `self.CurrentState` "NewEnumerator0"))))

(event `SpawnAttackActor`
  (params (IsSuperMove :type Boolean))
  (bind _returnvalue (`|SpawnActorFromClass` "/Game/_Game/Blueprints/Mutant/BP_MutantNormalAttack.BP_MutantNormalAttack_C" (`SceneComponent.GetSocketTransform` (`self.Mesh`) (select `bool` IsSuperMove :`false` (`self.AttackSocketName`) :`true` (`self.SuperMoveSocketName`)) "RTS_World") "Undefined" "MultiplyWithRoot" null (select `bool` IsSuperMove :`false` (`self.NormalAttackDamageNum`) :`true` (`self.SuperMoveDamageNum`)) self))
  (bind _output_get (set `self.AttackActor` _returnvalue))
  (`self.K2_AttachToComponent` _output_get (`self.Mesh`) (`self.AttackSocketName`) "SnapToTarget" "SnapToTarget" "SnapToTarget" true))

(event `RemoveAttackActor`
  (`self.K2_DestroyActor` (`self.AttackActor`)))

(fn `UserConstructionScript`
  (set `self.JumpMontage` null)
  (set `self.LightHittedMontage` "/Game/_Game/Assets/Animations/Mutant/Zombie_Reaction_Hit_Anim_Montage.Zombie_Reaction_Hit_Anim_Montage")
  (set `self.BigHittedMontage` "/Game/_Game/Assets/Animations/Mutant/Zombie_Reaction_Hit_Anim_Montage.Zombie_Reaction_Hit_Anim_Montage")
  (set `self.WinMontage` "/Game/_Game/Assets/Animations/Mutant/Victory_Anim_Montage.Victory_Anim_Montage")
  (set `self.LoseMontage` "/Game/_Game/Assets/Animations/Mutant/mutant_dying_Anim_Montage.mutant_dying_Anim_Montage")
  (set `self.AttackMontage` "/Game/_Game/Assets/Animations/Mutant/mutant_punch_Anim_Montage.mutant_punch_Anim_Montage")
  (set `self.SuperMoveMontage` "/Game/_Game/Assets/Animations/Mutant/mutant_swiping_Anim_Montage.mutant_swiping_Anim_Montage"))