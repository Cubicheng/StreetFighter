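; Base fighter character for a versus fighting game, turning each tick to face its Opponent.
; Attack, jump and block inputs are gated by a CurrentState enum, with montage completion returning the fighter to Idle.
; Blocking costs energy to start and hold, shows an overlay material and scales damage, while landed and received hits also adjust energy.
; Hits taken cause a stun montage or, at zero health, report the death to BP_FightingGameMode.
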(event `self.ReceiveBeginPlay`
  (set `self.Energy` 100.0)
  (set `self.Health` (`self.MaxHealth`)))

(event `self.ReceiveTick`
  (params (DeltaSeconds :type "Float (single-precision)"))
  (bind _opponent (`self.Opponent`))
  (bind (_returnvalue_roll _returnvalue_pitch _returnvalue_yaw) (`KismetMathLibrary.BreakRotator` (`KismetMathLibrary.FindLookAtRotation` (`self.K2_GetActorLocation`) (`self.K2_GetActorLocation` _opponent))))
  (`self.UpdateEnergy` DeltaSeconds)
  (if (`KismetSystemLibrary.IsValid` _opponent)
    (`self.K2_SetActorRotation` (`KismetMathLibrary.MakeRotator` 0.0 0.0 _returnvalue_yaw))))

(event `OnHit`
  (params (OtherIsBlocking :type Boolean))
  (if OtherIsBlocking
    (`self.AddEnergy` (`self.ENERGY GAIN ON HIT WITH BLOCK`))
    (else
      (`self.AddEnergy` (`self.ENERGY GAIN ON HIT WITH NO BLOCK`)))))

(event `PlayWinMontage`
  (`|PlayMontage` (`self.Mesh`) (`self.WinMontage`)))

(event `PlayLoseMontage`
  (`|PlayMontage` (`self.Mesh`) (`self.LoseMontage`)))

(event `EnhancedInput|/Game/Input/Actions/IA_Block`
  (params (ActionValue :type Boolean) (ElapsedSeconds :type "Float (double-precision)") (TriggeredSeconds :type "Float (double-precision)") (InputAction :type "InputAction Object Reference" :default "/Game/Input/Actions/IA_Block.IA_Block"))
  (:`Triggered`
    (bind _canblock (`self.CanBlock`))
    (if _canblock
      (`self.SetIsBlocking` true)
      (`self.AddEnergy` (* (`self.ENERGY COST ON BEGIN BLOCK`) -1.0))))
  (:`Completed`
    (`self.SetIsBlocking` false)))

(event `EnhancedInput|/Game/Input/Actions/IA_Jump`
  (params (ActionValue :type Boolean) (ElapsedSeconds :type "Float (double-precision)") (TriggeredSeconds :type "Float (double-precision)") (InputAction :type "InputAction Object Reference" :default "/Game/Input/Actions/IA_Jump.IA_Jump"))
  (:`Started`
    (bind _canjump (`self.CanChange2Jump`))
    (if _canjump
      (`self.SetIsBlocking` false)
      (set `self.CurrentState` "NewEnumerator4")
      (`self.SetIsBlocking` false)
      (`|PlayMontage` (`self.Mesh`) (`self.JumpMontage`)
        (:`OnCompleted`
          (set `self.CurrentState` "NewEnumerator0"))))))

(event `OnHitted`
  (params (DamageNum :type "Float (double-precision)"))
  (`self.UpdateEnergyOnHitted`)
  (if (`self.IsBlocking`)
    (bind _isdead (`self.UpdateHealth` (* DamageNum (`self.BlockDamageRate`))))
    (if (not _isdead)
      (set `self.CurrentState` "NewEnumerator3")
      (`|PlayMontage` (`self.Mesh`) (`self.LightHittedMontage`)
        (:`OnCompleted`
          _)
        (:`OnInterrupted`
          _))
      (set `self.CurrentState` "NewEnumerator0" :!label _label)
      (`self.SetIsBlocking` false))
    (else
      (bind _isdead_2 (`self.UpdateHealth` DamageNum))
      (if (not _isdead_2)
        (set `self.CurrentState` "NewEnumerator3")
        (`|PlayMontage` (`self.Mesh`) (`self.BigHittedMontage`)
          (:`OnCompleted`
            (goto _label))
          (:`OnInterrupted`
            (goto _label)))))))

(event `EnhancedInput|/Game/Input/Actions/IA_Attack`
  (params (ActionValue :type Boolean) (ElapsedSeconds :type "Float (double-precision)") (TriggeredSeconds :type "Float (double-precision)") (InputAction :type "InputAction Object Reference" :default "/Game/Input/Actions/IA_Attack.IA_Attack"))
  (:`Started`
    (bind _canattack (`self.CanAttack`))
    (if _canattack
      (`self.SetIsBlocking` false)
      (set `self.CurrentState` "NewEnumerator2")
      (`self.SetIsBlocking` false)
      (`|PlayMontage` (`self.Mesh`) (`self.AttackMontage`)
        (:`OnCompleted`
          (set `self.CurrentState` "NewEnumerator0"))))))

(fn `AddEnergy`
  (params (EnergyDelta :type "Float (double-precision)"))
  (returns (EnergyResult :type "Float (double-precision)"))
  (bind _returnvalue (+ (`self.Energy`) EnergyDelta))
  (if (>= _returnvalue (`self.MaxEnergy`))
    (bind _output_get (set `self.Energy` (`self.MaxEnergy`)))
    (return _output_get)
    (else
      (bind _output_get_2 (set `self.Energy` _returnvalue))
      (return _output_get_2))))

(fn `CanAttack`
  (returns (CanAttack :type Boolean))
  (switch `/Game/_Game/Blueprints/E_FightingState` (`self.CurrentState`)
    (:`NewEnumerator0`
      _)
    (:`NewEnumerator1`
      _)
    (:`NewEnumerator2`
      (return false))
    (:`NewEnumerator3`
      (return false))
    (:`NewEnumerator4`
      (return false)))
  (return true))

(fn `CanBlock`
  (returns (CanBlock :type Boolean))
  (if (`self.IsBlocking`)
    (return false)
    (elif (>= (`self.Energy`) (`self.ENERGY COST ON BEGIN BLOCK`))
      (switch `/Game/_Game/Blueprints/E_FightingState` (`self.CurrentState`)
        (:`NewEnumerator0`
          _)
        (:`NewEnumerator1`
          _)
        (:`NewEnumerator2`
          (return false))
        (:`NewEnumerator3`
          (return false))
        (:`NewEnumerator4`
          (return false)))
      (return true)
      (else
        (return false)))))

(fn `CanChange2Jump`
  (returns (CanJump :type Boolean))
  (switch `/Game/_Game/Blueprints/E_FightingState` (`self.CurrentState`)
    (:`NewEnumerator0`
      _)
    (:`NewEnumerator1`
      _)
    (:`NewEnumerator2`
      (return false))
    (:`NewEnumerator3`
      (return false))
    (:`NewEnumerator4`
      (return false)))
  (return true))

(fn `CanMove`
  (returns (CanMove :type Boolean))
  (switch `/Game/_Game/Blueprints/E_FightingState` (`self.CurrentState`)
    (:`NewEnumerator0`
      _)
    (:`NewEnumerator1`
      _)
    (:`NewEnumerator2`
      (return false))
    (:`NewEnumerator3`
      (return false))
    (:`NewEnumerator4`
      (return false)))
  (return true))

(fn `SetIsBlocking`
  (params (IsBlockingValue :type Boolean))
  (bind _output_get (set `self.IsBlocking` IsBlockingValue))
  (if _output_get
    (`MeshComponent.SetOverlayMaterial` (`self.Mesh`) "/Game/_Game/Assets/Materials/M_BlockHighlight.M_BlockHighlight")
    (else
      (`MeshComponent.SetOverlayMaterial` (`self.Mesh`) null))))

(fn `UpdateEnergy`
  (params (`Delta Seconds` :type "Float (double-precision)"))
  (if (`self.IsBlocking`)
    (bind _energyresult (`self.AddEnergy` (* (* `Delta Seconds` (`self.ENERGY COST ON BLOCKING PER SEC`)) -1.0)))
    (if (<= _energyresult 0.0)
      (set `self.Energy` 0.0)
      (`self.SetIsBlocking` false))))

(fn `UpdateEnergyOnHitted`
  (if (`self.IsBlocking`)
    (`self.AddEnergy` (`self.ENERGY GAIN ON HITTED WITH BLOCK`))
    (else
      (`self.AddEnergy` (`self.ENERGY GAIN ON HITTED WITH NO BLOCK`)))))

(fn `UpdateHealth`
  (params (Damage :type "Float (double-precision)"))
  (returns (IsDead :type Boolean))
  (bind _output_get (set `self.Health` (- (`self.Health`) Damage)))
  (if (<= _output_get 0.0)
    (`self.SetIsBlocking` false)
    (bind _asbp_fighting_game_mode (cast `/Game/_Game/Blueprints/BP_FightingGameMode` (`GameplayStatics.GetGameMode`)))
    (`/Game/_Game/Blueprints/BP_FightingGameMode.OnPlayerDied` _asbp_fighting_game_mode (`self.PlayerIndex`))
    (return true)
    (else
      (return false))))

(fn `UserConstructionScript`)