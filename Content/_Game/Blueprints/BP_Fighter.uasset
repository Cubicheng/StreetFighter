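; BP_Fighter is a player fighter character with stepping, a boxing attack and hit reactions, driven by Enhanced Input.
; A CurrentState enum (Idle, Moving, Attacking, Stunned) gates move and attack input, with montage callbacks returning it to Idle.
; MoveInput is adjusted by PlayerIndex and picks the forward or backward step montage.
; OnHitted stuns the fighter, and RegisterHitActor provides duplicate-hit filtering through HitActorList.
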(event `self.ReceiveBeginPlay`)

(event `self.ReceiveTick`
  (params (DeltaSeconds :type "Float (single-precision)"))
  (if (== (`self.PlayerIndex`) 0)
    (`KismetSystemLibrary.PrintString` (`|GetEnumeratorNameAsString` (`self.CurrentState`)))))

(event `EnhancedInput|/Game/Input/Actions/IA_Move`
  (params (ActionValue :type "Vector2D Structure") (ElapsedSeconds :type "Float (double-precision)") (TriggeredSeconds :type "Float (double-precision)") (InputAction :type "InputAction Object Reference" :default "/Game/Input/Actions/IA_Move.IA_Move"))
  (:`Triggered`
    (bind _canmove (`self.CanMove`))
    (if _canmove
      (bind _outputx (`self.CalcMoveInputByPlayerIndex` ActionValue_X))
      (bind _output_get (set `self.MoveInput` _outputx))
      (if (`|EnumEquality` (`self.CurrentState`) "NewEnumerator0")
        (set `self.CurrentState` "NewEnumerator1")
        (if (> _output_get 0.0) :!label _label
          (`|PlayMontage` (`self.Mesh`) "/Game/_Game/Assets/Animations/Short_Step_Forward_Anim_Montage.Short_Step_Forward_Anim_Montage" 1.5
            (:`OnCompleted`
              _))
          (else
            (`|PlayMontage` (`self.Mesh`) "/Game/_Game/Assets/Animations/Step_Backward_Anim_Montage.Step_Backward_Anim_Montage"
              (:`OnCompleted`
                _))))
        (set `self.CurrentState` "NewEnumerator0"))))
  (:`Started`
    (bind _canmove_2 (`self.CanMove`))
    (if _canmove_2
      (goto _label)))
  (:`Completed`
    (`self.StopAnimMontage` "/Game/_Game/Assets/Animations/Step_Backward_Anim_Montage.Step_Backward_Anim_Montage")
    (`self.StopAnimMontage` "/Game/_Game/Assets/Animations/Short_Step_Forward_Anim_Montage.Short_Step_Forward_Anim_Montage")
    (set `self.CurrentState` "NewEnumerator0")))

(event `EnhancedInput|/Game/Input/Actions/IA_Attack`
  (params (ActionValue :type Boolean) (ElapsedSeconds :type "Float (double-precision)") (TriggeredSeconds :type "Float (double-precision)") (InputAction :type "InputAction Object Reference" :default "/Game/Input/Actions/IA_Attack.IA_Attack"))
  (:`Started`
    (bind _canattack (`self.CanAttack`))
    (if _canattack
      (set `self.CurrentState` "NewEnumerator2")
      (`|PlayMontage` (`self.Mesh`) "/Game/_Game/Assets/Animations/Boxing_Anim_Montage.Boxing_Anim_Montage"
        (:`OnCompleted`
          (set `self.CurrentState` "NewEnumerator0"))))))

(event `OnHitted`
  (`KismetSystemLibrary.PrintString` "hit")
  (set `self.CurrentState` "NewEnumerator3")
  (`|PlayMontage` (`self.Mesh`) "/Game/_Game/Assets/Animations/Hit_To_Body_Anim_Montage.Hit_To_Body_Anim_Montage"
    (:`OnCompleted`
      _)
    (:`OnInterrupted`
      _))
  (set `self.CurrentState` "NewEnumerator0"))

(fn `CalcMoveInputByPlayerIndex`
  (params (inputX :type "Float (double-precision)"))
  (returns (outputX :type "Float (double-precision)"))
  (if (== (`self.PlayerIndex`) 0)
    (return inputX)
    (else
      (bind _result (`/Engine/EditorBlueprintResources/StandardMacros.NegateFloat` inputX)
        (:`  `
          (return _result))))))

(fn `CanAttack`
  (returns (CanAttack :type Boolean))
  (switch `/Game/_Game/Blueprints/E_FighterState` (`self.CurrentState`)
    (:`NewEnumerator0`
      _)
    (:`NewEnumerator1`
      _)
    (:`NewEnumerator2`
      (return false))
    (:`NewEnumerator3`
      (return false)))
  (return true))

(fn `CanMove`
  (returns (CanMove :type Boolean))
  (switch `/Game/_Game/Blueprints/E_FighterState` (`self.CurrentState`)
    (:`NewEnumerator0`
      _)
    (:`NewEnumerator1`
      _)
    (:`NewEnumerator2`
      (return false))
    (:`NewEnumerator3`
      (return false)))
  (return true))

(fn `RegisterHitActor`
  (params (TargetActor :type "Actor Object Reference"))
  (returns (IsNewHit :type Boolean))
  (if (`KismetArrayLibrary.Array_Contains` (`self.HitActorList`) TargetActor)
    (return false)
    (else
      (`KismetArrayLibrary.Array_Add` (`self.HitActorList`) TargetActor)
      (return true))))

(fn `UserConstructionScript`)