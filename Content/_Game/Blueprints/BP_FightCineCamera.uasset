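; Fighting game cine camera that keeps the first two players framed during one specific game mode state.
; OnEnterFight caches the game mode and its player list.
; Each tick, the actor eases toward the players' midpoint in Y and Z, keeping its X.
; As their distance grows, clamped range mapping pulls the camera component back along local X and shortens focal length, both interpolated.
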(event `self.ReceiveTick`
  (params (DeltaSeconds :type "Float (single-precision)"))
  (bind _returnvalue_x (`KismetMathLibrary.BreakVector` (`self.K2_GetActorLocation`)))
  (bind (_targety _targetz) (`self.GetTargetYZ` DeltaSeconds))
  (bind _fightcinecamera (`self.FightCineCamera`))
  (bind _bp_fighting_game_mode (`self.BP Fighting Game Mode`))
  (bind _returnvalue (`SceneComponent.GetRelativeTransform` _fightcinecamera))
  (if (`KismetSystemLibrary.IsValid` _bp_fighting_game_mode)
    (if (`|EnumEquality` (`/Game/_Game/Blueprints/BP_FightingGameMode.E_GameState` _bp_fighting_game_mode) "NewEnumerator2")
      (`self.K2_SetActorLocation` (`KismetMathLibrary.MakeVector` _returnvalue_x _targety _targetz))
      (`SceneComponent.K2_SetRelativeLocation` _fightcinecamera (`KismetMathLibrary.MakeVector` (`self.GetTargetX` DeltaSeconds) (.y (.location _returnvalue)) (.z (.location _returnvalue))) false false)
      (set `CineCameraComponent.CurrentFocalLength` (`self.GetTargetFocal` DeltaSeconds) (`self.FightCineCamera`)))))

(event `OnEnterFight`
  (bind _asbp_fighting_game_mode (cast `/Game/_Game/Blueprints/BP_FightingGameMode` (`GameplayStatics.GetGameMode`)))
  (bind _output_get (set `self.BP Fighting Game Mode` _asbp_fighting_game_mode))
  (set `self.PlayerList` (`/Game/_Game/Blueprints/BP_FightingGameMode.PlayerList` _output_get)))

(fn `GetTargetFocal`
  (params (deltaTime :type "Float (double-precision)"))
  (returns (targetFocal :type "Float (double-precision)"))
  (bind _playerlist (`self.PlayerList`))
  (return (`KismetMathLibrary.FInterpTo` (`CineCameraComponent.CurrentFocalLength` (`self.FightCineCamera`)) (`KismetMathLibrary.MapRangeClamped` (`self.GetDistanceTo` (`|GetArrayItem` _playerlist) (`|GetArrayItem` _playerlist 1)) 200.0 1500.0 24.0 12.0) deltaTime 53.0)))

(fn `GetTargetX`
  (params (deltaTime :type "Float (double-precision)"))
  (returns (targetX :type "Float (double-precision)"))
  (bind _playerlist (`self.PlayerList`))
  (bind _relativelocation_x (`KismetMathLibrary.BreakVector` (`SceneComponent.RelativeLocation` (`self.FightCineCamera`))))
  (return (`KismetMathLibrary.FInterpTo` _relativelocation_x (`KismetMathLibrary.MapRangeClamped` (`self.GetDistanceTo` (`|GetArrayItem` _playerlist) (`|GetArrayItem` _playerlist 1)) 200.0 1500.0 0.0 -500.0) deltaTime 5.0)))

(fn `GetTargetYZ`
  (params (deltaTime :type "Float (double-precision)"))
  (returns (targetY :type "Float (double-precision)") (targetZ :type "Float (double-precision)"))
  (bind _playerlist (`self.PlayerList`))
  (bind (_returnvalue_x _returnvalue_y _returnvalue_z) (`KismetMathLibrary.BreakVector` (`KismetMathLibrary.VInterpTo` (`self.K2_GetActorLocation`) (* (+ (`self.K2_GetActorLocation` (`|GetArrayItem` _playerlist)) (`self.K2_GetActorLocation` (`|GetArrayItem` _playerlist 1))) (0.5 0.5 0.5)) deltaTime 5.0)))
  (return _returnvalue_y _returnvalue_z))

(fn `UserConstructionScript`)