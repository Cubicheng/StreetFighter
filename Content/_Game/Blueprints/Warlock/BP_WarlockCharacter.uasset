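; Warlock character Blueprint that handles movement input and supplies the Warlock's animation montages to inherited character logic.
; The construction script assigns montages for jump, light and heavy hit reactions, win, lose and attack.
; IA_Move applies single-axis input along a fixed diagonal world direction when CanMove passes, or while falling otherwise.
; Permitted movement sets CurrentState, and releasing input reverts it only if still in that movement state.
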(event `self.ReceiveBeginPlay`
  (`parent.ReceiveBeginPlay`))

(event `self.ReceiveTick`
  (params (DeltaSeconds :type "Float (single-precision)"))
  (`parent.ReceiveTick` DeltaSeconds))

(event `EnhancedInput|/Game/Input/Actions/IA_Move`
  (params (ActionValue :type "Vector2D Structure") (ElapsedSeconds :type "Float (double-precision)") (TriggeredSeconds :type "Float (double-precision)") (InputAction :type "InputAction Object Reference" :default "/Game/Input/Actions/IA_Move.IA_Move"))
  (:`Triggered`
    (bind _canmove (`self.CanMove`))
    (if _canmove
      (`self.AddMovementInput` (1.0 1.0 1.0) ActionValue_X)
      (set `self.CurrentState` "NewEnumerator1")
      (if (<= ActionValue_X 0.0)
        _)
      (elif (`NavMovementComponent.IsFalling` (`self.CharacterMovement`))
        (`self.AddMovementInput` (1.0 1.0 0.0) ActionValue_X))))
  (:`Completed`
    (if (`|EnumEquality` (`self.CurrentState`) "NewEnumerator1")
      (set `self.CurrentState` "NewEnumerator0"))))

(fn `UserConstructionScript`
  (set `self.JumpMontage` "/Game/_Game/Assets/Animations/Warlock/Standing_Jump_Anim_Montage.Standing_Jump_Anim_Montage")
  (set `self.LightHittedMontage` "/Game/_Game/Assets/Animations/Warlock/Standing_React_Small_From_Front_Anim_Montage.Standing_React_Small_From_Front_Anim_Montage")
  (set `self.BigHittedMontage` "/Game/_Game/Assets/Animations/Warlock/Standing_React_Large_From_Front_Anim_Montage.Standing_React_Large_From_Front_Anim_Montage")
  (set `self.WinMontage` "/Game/_Game/Assets/Animations/Ninja/Victory_Anim_Montage.Victory_Anim_Montage")
  (set `self.LoseMontage` "/Game/_Game/Assets/Animations/Warlock/Standing_React_Death_Backward_Anim_Montage.Standing_React_Death_Backward_Anim_Montage")
  (set `self.AttackMontage` "/Game/_Game/Assets/Animations/Warlock/Standing_1H_Magic_Attack_01_Anim_Montage.Standing_1H_Magic_Attack_01_Anim_Montage"))